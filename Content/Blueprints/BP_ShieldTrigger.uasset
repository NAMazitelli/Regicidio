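; BP_ShieldTrigger is a one-shot trigger that raises a shield when a player-tagged actor overlaps it.
; On activation it reveals and activates its linked crystals, counts them, and spawns a BP_Shield at its root location.
; It listens to each crystal's destroyed event and, once none remain, destroys both the shield and itself.
; The SetActorDisabled function is an empty stub.
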(event Custom|activateShield
  (Variables|Default|SetisActive true)
  (for _array_element (Variables|Default|GetCristals)
    (Variables|/Game/Blueprints/BP_Cristal.BP_Cristal_C|SetisActive _array_element true)
    (Variables|Default|SetActiveCristals (+ (Variables|Default|GetActiveCristals) 1))
    (Rendering|SetActorHiddenInGame _array_element false)
    (Game|BindEventtoOnDestroyed _array_element (delegate Custom|CustomEvent_0)))
  (bind _returnvalue (Game|SpawnActorfromClass "/Game/Blueprints/BP_Shield.BP_Shield_C" (Math|Transform|MakeTransform (Transformation|GetWorldLocation (Variables|Default|GetDefaultSceneRoot))) "Undefined" 0 0))
  (Variables|Default|SetShield _returnvalue))

(event Custom|CustomEvent_0
  (params (DestroyedActor :type Actor%20Object%20Reference))
  (bind _output_get (Variables|Default|SetActiveCristals (- (Variables|Default|GetActiveCristals) 1)))
  (if (<= _output_get 0)
    (Actor|DestroyActor (Variables|Default|GetShield))
    (Actor|DestroyActor)))

(event EventBeginPlay)

(event Collision|EventActorBeginOverlap
  (params (OtherActor :type Actor%20Object%20Reference))
  (if (Actor|ActorHasTag OtherActor "player")
    (if (not (Variables|Default|GetisActive))
      (Variables|Default|SetisActive true)
      (CallFunction|ActivateShield))))

(fn ConstructionScript)

(fn SetActorDisabled
  (params (actor :type Actor%20Object%20Reference) (isactive :type Boolean)))