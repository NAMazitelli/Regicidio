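; BP_bullet is a side-colored projectile that damages only enemies vulnerable to the weapon side that fired it.
; On spawn it tints a dynamic material with its Color and launches the mesh with a physics impulse along its arrow's forward vector.
; On overlap it ignores Weapon-tagged actors, applies damage when an EnemyTemplate's KilledBySide matches WeaponSide, and destroys itself.
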(event EventBeginPlay
  ;[1 1 1] Send forward on spawn
  (bind _returnvalue (Rendering|Material|CreateDynamicMaterialInstance (Variables|Default|GetbulletMesh) 0 "/Game/Materials/WeaponsMaterial.WeaponsMaterial" "None" :!class /Script/Engine.PrimitiveComponent))
  (Rendering|Material|SetVectorParameterValue _returnvalue "DiffuseColor" (Variables|Default|GetColor) :!class /Script/Engine.MaterialInstanceDynamic)
  (Physics|AddImpulse (Variables|Default|GetbulletMesh) (* (Math|Vector|GetForwardVector (Variables|Default|GetArrowRef)) 500) "None" false))

(event Collision|EventActorBeginOverlap
  (params (OtherActor :type Actor%20Object%20Reference))
  ;[1 1 1] Destroy on overlap with anything that's not tagged as weapon
  (if (not (Actor|ActorHasTag OtherActor "Weapon"))
    (if (Actor|ActorHasTag OtherActor "Enemy")
      (bind _asenemy_template (Utilities|Casting|CastToEnemyTemplate OtherActor))
      (if (== (Variables|/Game/Blueprints/Characters/Zombie/EnemyTemplate.EnemyTemplate_C|GetKilledBySide _asenemy_template) (Variables|Default|GetWeaponSide))
        (Game|Damage|ApplyDamage OtherActor 1e+01 0 0)))
    (Actor|DestroyActor)))

(fn ConstructionScript)