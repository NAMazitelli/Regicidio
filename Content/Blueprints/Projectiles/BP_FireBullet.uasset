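; BP_FireBullet is a projectile that deals fixed damage to actors tagged "player" on overlap.
; It destroys itself after that damage or on overlapping anything else, except actors tagged "bullet", which it ignores.
; The forward impulse on its Sphere is disconnected and BeginPlay is empty, so this graph does not launch it.
; The Hit event only prints a debug string and has an empty player-tag branch.
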(event EventBeginPlay
  ;[1 1 1] Send forward on spawn
)

(event Collision|EventHit
  (params (MyComp :type Primitive%20Component%20Object%20Reference) (Other :type Actor%20Object%20Reference) (OtherComp :type Primitive%20Component%20Object%20Reference) (bSelfMoved :type Boolean) (HitLocation :type Vector :default "0, 0, 0") (HitNormal :type Vector :default "0, 0, 0") (NormalImpulse :type Vector :default "0, 0, 0") (Hit :type Hit%20Result%20Structure%20%28by%20ref%29))
  (Development|PrintString "Hello")
  (if (Actor|ActorHasTag Other "player")
    _))

(event Collision|EventActorBeginOverlap
  (params (OtherActor :type Actor%20Object%20Reference))
  ;[1 1 1] Destroy on overlap with anything that's not tagged as weapon
  (if (Actor|ActorHasTag OtherActor "player")
    (Game|Damage|ApplyDamage OtherActor 1e+01 0 0)
    (Actor|DestroyActor :!label _label)
    (elif (not (Actor|ActorHasTag OtherActor "bullet"))
      (goto _label))))

(fn ConstructionScript)