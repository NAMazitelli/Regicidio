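; VR game mode that spawns and possesses the player pawn at the selected start point when play begins.
; It matches BP_PlayerStart actors against the start number in GameInstanceVR settings, storing the match's transform and play-as-PC flag there.
; That flag selects FirstPersonCharacter or MotionControllerPawn; a spawned BPP_Pawn receives the settings.
; SpawnDefaultPawnFor is overridden to return nothing, leaving spawning to this logic.
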(event Custom|GetPlayerStartData
  (for _array_element (Variables|Default|GetBP_PlayerStart)
    (if (== (Variables|/Game/Blueprints/Dev/BP_PlayerStart.BP_PlayerStart_C|GetStartNumber _array_element) (.PlayerStartNumber (Utilities|Struct|BreakStruc_VRPlayerSettings (Variables|/Game/Blueprints/Core/GameInstanceVR.GameInstanceVR_C|GetStruc%20VR%20Player%20Settings (Variables|References|GetGame%20Instance)))))
      (Utilities|Struct|SetmembersinStruc_VRPlayerSettings (Variables|/Game/Blueprints/Core/GameInstanceVR.GameInstanceVR_C|GetStruc%20VR%20Player%20Settings (Variables|References|GetGame%20Instance)) (Variables|/Game/Blueprints/Dev/BP_PlayerStart.BP_PlayerStart_C|GetPlayAsPC _array_element) (Transformation|GetActorTransform _array_element)))))

(event Custom|SpawnActorToMap
  (bind _returnvalue (Game|GetPlayerController 0))
  (bind _game_instance (Variables|References|GetGame%20Instance))
  (bind _struc_vr_player_settings (Variables|/Game/Blueprints/Core/GameInstanceVR.GameInstanceVR_C|GetStruc%20VR%20Player%20Settings _game_instance))
  (bind (_testingmode _spawntransform) (Utilities|Struct|BreakStruc_VRPlayerSettings _struc_vr_player_settings))
  ;[1 1 1] Spawn actor to map
  (bind _aspawn (Utilities|Casting|CastToPawnClass (select _testingmode "/Game/Blueprints/Characters/PCPawn/FirstPersonCharacter.FirstPersonCharacter_C" "/Game/Blueprints/Characters/VRPawn/MotionControllerPawn.MotionControllerPawn_C")))
  (bind _returnvalue_2 (Game|SpawnActorfromClass _aspawn _spawntransform "AlwaysSpawn" _returnvalue 0))
  (Pawn|Possess _returnvalue _returnvalue_2)
  (bind _asbpp_pawn (Utilities|Casting|CastToBPP_Pawn _returnvalue_2))
  (Variables|/Game/Blueprints/Characters/ParentPawn/BPP_Pawn.BPP_Pawn_C|SetStruc_VRPlayerSettings _asbpp_pawn (Variables|/Game/Blueprints/Core/GameInstanceVR.GameInstanceVR_C|GetStruc%20VR%20Player%20Settings (Variables|References|GetGame%20Instance))))

(event EventBeginPlay
  (bind _asgame_instance_vr (Utilities|Casting|CastToGameInstanceVR (Game|GetGameInstance)))
  ;[1 1 1] Get reference to gameinstance
  (Variables|References|SetGame%20Instance _asgame_instance_vr)
  ;[1 1 1] get all pawns
  (bind _outactors (Actor|GetAllActorsOfClass "/Game/Blueprints/Dev/BP_PlayerStart.BP_PlayerStart_C"))
  (Variables|Default|SetBP_PlayerStart _outactors)
  (CallFunction|GetPlayerStartData)
  (CallFunction|SpawnActortoMap))

(event EventTick
  (params (DeltaSeconds :type Float%20%28single-precision%29)))

(fn ConstructionScript)

(fn SpawnDefaultPawnfor
  (params (NewPlayer :type Controller%20Object%20Reference) (StartSpot :type Actor%20Object%20Reference))
  (return 0))