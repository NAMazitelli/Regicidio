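; Enemy shooter actor that turns to face the player and fires BP_FireBullet projectiles at a fixed interval.
; Tick aims at the VR pawn's camera, or at a raised player location when the player's TestingMode setting is on.
; BeginPlay starts a delay loop that spawns bullets from the Arrow's transform and ends once IsFiring is false.
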(event Custom|Fire
  (bind _arrow (Variables|Default|GetArrow))
  ;[1 1 1] spawn projectile logic
  (bind _returnvalue (Game|SpawnActorfromClass "/Game/Blueprints/Projectiles/BP_FireBullet.BP_FireBullet_C" (Math|Transform|MakeTransform (Transformation|GetWorldLocation _arrow) (Transformation|GetWorldRotation _arrow) "1,1,1") "AlwaysSpawn" 0 0 "NewEnumerator0" "(R=0.000000,G=0.000000,B=0.000000,A=0.000000)" 0)))

(event EventBeginPlay
  (if (Variables|Default|GetisFiring) :!label _label
    (CallFunction|Fire)
    (Utilities|FlowControl|RetriggerableDelay 0.5)
    (goto _label)))

(event Collision|EventActorBeginOverlap
  (params (OtherActor :type Actor%20Object%20Reference)))

(event EventTick
  (params (DeltaSeconds :type Float%20%28single-precision%29))
  (bind _returnvalue (Game|GetPlayerCharacter 0))
  (bind _defaultsceneroot (Variables|Default|GetDefaultSceneRoot))
  (bind _returnvalue_2 (Transformation|GetActorLocation _returnvalue))
  (bind _relativelocation (Variables|/Script/Engine.SceneComponent|GetRelativeLocation _defaultsceneroot))
  (bind _asbpp_pawn (Utilities|Casting|CastToBPP_Pawn _returnvalue))
  (if (.TestingMode (Utilities|Struct|BreakStruc_VRPlayerSettings (Variables|/Game/Blueprints/Characters/ParentPawn/BPP_Pawn.BPP_Pawn_C|GetStruc_VRPlayerSettings _asbpp_pawn)))
    (Transformation|SetActorRotation (Math|Rotator|FindLookatRotation (Math|Vector|MakeVector (.x _relativelocation) (.y _relativelocation) (.z _relativelocation)) (Math|Vector|MakeVector (.x _returnvalue_2) (.y _returnvalue_2) (+ (.z _returnvalue_2) 3e+01 0.0))))
    (else
      (bind _asmotion_controller_pawn (Utilities|Casting|CastToMotionControllerPawn _returnvalue))
      (Transformation|SetActorRotation (Math|Rotator|FindLookatRotation (Variables|/Script/Engine.SceneComponent|GetRelativeLocation (Variables|Default|GetDefaultSceneRoot)) (Transformation|GetWorldLocation (Variables|/Game/Blueprints/Characters/VRPawn/MotionControllerPawn.MotionControllerPawn_C|GetCamera _asmotion_controller_pawn)))))))

(fn ConstructionScript)