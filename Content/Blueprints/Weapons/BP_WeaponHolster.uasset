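; Weapon holster actor for a left or right side that spawns a pickup weapon and keeps it beside the player's camera.
; On BeginPlay it spawns a BP_PickupWeapon with the matching side, snaps it to the Holster component and rotates it 180 degrees.
; Tick sets the root's relative location from the camera's, offset forward and sideways by Side.
; The construction script shifts the Holster by the same Y offset for both sides.
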(event EventBeginPlay
  ;[1 1 1] spawn weapons
  (bind _returnvalue (Game|SpawnActorfromClass "/Game/Blueprints/Weapons/BP_PickupWeapon.BP_PickupWeapon_C" (Math|Transform|MakeTransform "0, 0, 0") "AlwaysSpawn" self (Variables|Default|GetSide) 0))
  (Transformation|AttachComponentToComponent _returnvalue (Variables|Default|GetHolster) "None" "SnapToTarget" "KeepRelative" "KeepRelative" false)
  (Transformation|SetRelativeRotation (Variables|/Script/Engine.Actor|GetRootComponent _returnvalue) "0.000000,180.000000,0.000000" false false))

(event EventTick
  (params (DeltaSeconds :type Float%20%28single-precision%29))
  (bind _defaultsceneroot (Variables|Default|GetDefaultSceneRoot))
  (bind _cameraref (Variables|Default|GetCameraRef))
  (bind _relativelocation (Variables|/Script/Engine.SceneComponent|GetRelativeLocation _cameraref))
  (bind _relativelocation_2 (Variables|/Script/Engine.SceneComponent|GetRelativeLocation _cameraref))
  ;[1 1 1] stick to camera
  (switch Utilities|FlowControl|Switch|SwitchonEWeaponHolster (Variables|Default|GetSide)
    (:NewEnumerator0
      (Transformation|SetRelativeLocation _defaultsceneroot (Math|Vector|MakeVector (+ (.x _relativelocation) 25.0) (- (.y _relativelocation) 2e+01) (.z _relativelocation)) false false))
    (:NewEnumerator1
      (Transformation|SetRelativeLocation _defaultsceneroot (Math|Vector|MakeVector (+ (.x _relativelocation_2) 25.0) (+ (.y _relativelocation_2) 2e+01) (.z _relativelocation_2)) false false))))

(fn ConstructionScript
  (bind _holster (Variables|Default|GetHolster))
  (switch Utilities|FlowControl|Switch|SwitchonEWeaponHolster (Variables|Default|GetSide)
    (:NewEnumerator0
      (Class|SceneComponent|AddLocalTransform _holster (Math|Transform|MakeTransform "0.000000,-60.000000,0.000000") false true))
    (:NewEnumerator1
      (Class|SceneComponent|AddLocalTransform _holster (Math|Transform|MakeTransform "0.000000,-60.000000,0.000000") false true))))