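; Pickup gun actor that BP_MotionController attaches on Pickup and that snaps back to the BP_WeaponHolster matching its WeaponSide on Drop.
; ShootEvent runs Shoot, a hitscan trace from the Arrow that spawns a short-lived impact decal.
; Shoot plays animation, sound and muzzle flash, then calls shootAnimation, which repeats them and hides the flash after a delay.
; Laser pointer, side-based tinting and projectile spawning exist but are unwired.
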(event Custom|ShootEvent
  (CallFunction|Shoot))

(event Custom|shootAnimation
  (Components|Animation|PlayAnimation (Variables|SkeletalMeshActor|GetSkeletalMeshComponent) "/Game/Meshes/Weapons/ImperiaGun/ImperiaGun_Shoot.ImperiaGun_Shoot" false)
  (Audio|PlaySoundatLocation "/Game/Sounds/Sound_Shoot_Cue.Sound_Shoot_Cue" (Transformation|GetActorLocation) "0, 0, 0" 1.0 1.0 0.0 0 0 0)
  (Rendering|SetVisibility (Variables|Default|GetMuzzle) true false)
  (Utilities|FlowControl|Delay 0.1)
  (Rendering|SetVisibility (Variables|Default|GetMuzzle) false false))

(event EventBeginPlay)

(event Collision|EventActorBeginOverlap
  (params (OtherActor :type Actor%20Object%20Reference)))

(event EventTick
  (params (DeltaSeconds :type Float%20%28single-precision%29)))

(event EventPickup
  (params (AttachTo :type Scene%20Component%20Object%20Reference) (Location :type Transform))
  (bind _returnvalue (VehicleSound|GetRootComponent))
  (bind (_location _rotation) (Math|Transform|BreakTransform Location))
  (Physics|SetSimulatePhysics (Variables|SkeletalMeshActor|GetSkeletalMeshComponent) false)
  (Transformation|AttachComponentToComponent _returnvalue AttachTo "None" "SnapToTarget" "SnapToTarget" "KeepWorld" false)
  (Transformation|SetRelativeLocationAndRotation _returnvalue _location _rotation false false))

(event EventDrop
  (Transformation|DetachFromActor "KeepWorld" "KeepWorld" "KeepWorld")
  (bind _outactors (Actor|GetAllActorsOfClass "/Game/Blueprints/Weapons/BP_WeaponHolster.BP_WeaponHolster_C"))
  (for _array_element _outactors
    (if (== (Variables|/Game/Blueprints/Weapons/BP_WeaponHolster.BP_WeaponHolster_C|GetSide _array_element) (Variables|Default|GetWeaponSide))
      (Transformation|AttachActorToActor _array_element "None" "SnapToTarget" "SnapToTarget" "KeepWorld" false)
      (Transformation|SetRelativeLocationAndRotation (VehicleSound|GetRootComponent) (Variables|/Script/Engine.SceneComponent|GetRelativeLocation (Variables|/Game/Blueprints/Weapons/BP_WeaponHolster.BP_WeaponHolster_C|GetHolster _array_element)) "0.000000,-90.000000,90.000000" false true))))

(fn ConstructionScript)

(fn Shoot
  (bind _arrow (Variables|Default|GetArrow))
  (bind _returnvalue (Transformation|GetSocketLocation _arrow "None"))
  (bind _outhit (Collision|LineTraceByChannel _returnvalue (+ _returnvalue (* (Math|Vector|GetForwardVector (Variables|Default|GetArrow)) 2.5e+04)) "TraceTypeQuery1" false 0 "None" true "(R=1.000000,G=0.000000,B=0.000000,A=1.000000)" "(R=0.000000,G=1.000000,B=0.000000,A=1.000000)" 1.0))
  (Class|GameplayStatics|SpawnDecalAttached "/Game/Materials/Textures/T_Impact_Mask_Mat_Inst.T_Impact_Mask_Mat_Inst" "30.000000,30.000000,30.000000" (.HitComponent (Collision|BreakHitResult _outhit)) "None" (.ImpactPoint (Collision|BreakHitResult _outhit)) (Math|Conversions|RotationFromXVector (.ImpactNormal (Collision|BreakHitResult _outhit))) "KeepWorldPosition" 3.0)
  (Components|Animation|PlayAnimation (Variables|SkeletalMeshActor|GetSkeletalMeshComponent) "/Game/Meshes/Weapons/ImperiaGun/ImperiaGun_Shoot.ImperiaGun_Shoot" false)
  (Audio|PlaySoundatLocation "/Game/Sounds/Sound_Shoot_Cue.Sound_Shoot_Cue" (Transformation|GetActorLocation) "0, 0, 0" 1.0 1.0 0.0 0 0 0)
  (Rendering|SetVisibility (Variables|Default|GetMuzzle) true false)
  (CallFunction|ShootAnimation))

(fn DrawLaser
  (bind _arrow (Variables|Default|GetArrow))
  (bind _returnvalue (Transformation|GetWorldLocation _arrow))
  ;[1 1 1] Draw Laser
  (if (Variables|Default|GetisLaserActive)
    (if (Utilities|IsValid (Variables|Default|GetMenuLaser))
      _
      (else
        (bind _returnvalue_2 (Effects|SpawnEmitterAttached "/Game/FX/LaserRay/PS_LaserRay.PS_LaserRay" (Variables|Default|GetArrow) "None"))
        (Variables|Default|SetMenuLaser _returnvalue_2)))
    (Class|ParticleSystemComponent|SetBeamSourcePoint (Variables|Default|GetMenuLaser) 0 _returnvalue)
    (bind _outhit (Collision|LineTraceByChannel _returnvalue (+ (* (Math|Vector|GetForwardVector _arrow) 2e+03) _returnvalue) "TraceTypeQuery1" false 0 "None"))
    (Class|ParticleSystemComponent|SetBeamTargetPoint (Variables|Default|GetMenuLaser) 0 (Math|Vector|SelectVector (.Location (Collision|BreakHitResult _outhit)) (.TraceEnd (Collision|BreakHitResult _outhit)) (.bBlockingHit (Collision|BreakHitResult _outhit))))
    (if (.bBlockingHit (Collision|BreakHitResult _outhit))
      _)
    (elif (Utilities|IsValid (Variables|Default|GetMenuLaser))
      (Components|DestroyComponent (Variables|Default|GetMenuLaser)))))