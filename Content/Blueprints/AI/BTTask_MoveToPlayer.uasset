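; Behavior tree task that sends a boss pawn toward the player when the player is within a set range.
; An inactive boss first holds a battlecry flag through a short delay, then turns active and writes that to the blackboard.
; AI MoveTo success or an out-of-range player finishes the task successfully, while a failed move has no finish path.
; Abort stops the controller's movement.
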(event EventReceiveAbort
  (params (OwnerActor :type Actor%20Object%20Reference))
  (AI|Navigation|StopMovement (Variables|Default|GetAi%20Reference))
  (Class|BTTaskBlueprintBase|FinishAbort))

(event EventReceiveExecuteAI
  (params (OwnerController :type AI%20Controller%20Object%20Reference) (ControlledPawn :type Pawn%20Object%20Reference))
  (bind _returnvalue (Game|Player|GetPlayerPawn 0))
  (Variables|Default|SetAi%20Reference OwnerController)
  (if (< (Math|Vector|VectorLength (- (Transformation|GetActorLocation _returnvalue) (Transformation|GetActorLocation ControlledPawn))) 7e+03)
    (bind _asboss_template (Utilities|Casting|CastToBossTemplate ControlledPawn))
    (if (Variables|/Game/Blueprints/Characters/Bucefalo/BossTemplate.BossTemplate_C|GetisActive _asboss_template)
      _
      (else
        (Variables|/Game/Blueprints/Characters/Bucefalo/BossTemplate.BossTemplate_C|SetisBattlecry _asboss_template true)
        (Utilities|FlowControl|Delay 2.7)
        (Variables|/Game/Blueprints/Characters/Bucefalo/BossTemplate.BossTemplate_C|SetisBattlecry _asboss_template false)
        (bind _output_get (Variables|/Game/Blueprints/Characters/Bucefalo/BossTemplate.BossTemplate_C|SetisActive _asboss_template true))
        (Class|BTFunctionLibrary|SetBlackboardValueasBool (Variables|Default|GetisActive) _output_get)))
    (AI|AIMoveTo _asboss_template "0, 0, 0" _returnvalue 1e+02 true
      (:OnSuccess
        _)))
  (AI|BehaviorTree|FinishExecute true))