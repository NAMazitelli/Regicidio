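; Behavior Tree service that flags whether the AI should be attacking, based on its distance to the player.
; On each tick it measures the distance between the controlled pawn and the first player pawn.
; It sets the IsAttacking blackboard key true within a fixed 2000-unit range and false otherwise.
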(event EventTick
  (params (OwnerActor :type Actor%20Object%20Reference) (DeltaSeconds :type Float%20%28single-precision%29))
  (bind _isattacking (Variables|Default|GetisAttacking))
  (if (< (Math|Vector|VectorLength (- (Transformation|GetActorLocation (Pawn|GetControlledPawn (AI|GetAIController OwnerActor))) (Transformation|GetActorLocation (Game|Player|GetPlayerPawn 0)))) 2e+03)
    (Class|BTFunctionLibrary|SetBlackboardValueasBool _isattacking true)
    (else
      (Class|BTFunctionLibrary|SetBlackboardValueasBool _isattacking false))))